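; Ambient sound actor that plays audio only while the VR player is inside its area.
; When a VRPawn begins overlapping the Area component, the AmbientSound fades in over a few seconds, and it fades out the same way when the pawn leaves.
; Other actors are ignored through the cast to VRPawn, and Tick and the construction script do nothing.
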(event `self.Area.OnComponentBeginOverlap`
  (params (OverlappedComponent :type "PrimitiveComponent Object Reference") (OtherActor :type "Actor Object Reference") (OtherComp :type "PrimitiveComponent Object Reference") (OtherBodyIndex :type Integer) (bFromSweep :type Boolean) (SweepResult :type "HitResult Structure (by ref)"))
  ;[1 1 1] Fade in
  (bind _asvrpawn (cast `/Game/VRTemplate/Blueprints/VRPawn` OtherActor))
  (if (== OtherActor _asvrpawn)
    (`AudioComponent.FadeIn` (`self.AmbientSound`) 3.0 1.0 0.0 "Linear")))

(event `self.Area.OnComponentEndOverlap`
  (params (OverlappedComponent :type "PrimitiveComponent Object Reference") (OtherActor :type "Actor Object Reference") (OtherComp :type "PrimitiveComponent Object Reference") (OtherBodyIndex :type Integer))
  ;[1 1 1] Fade out
  (bind _asvrpawn (cast `/Game/VRTemplate/Blueprints/VRPawn` OtherActor))
  (if (== OtherActor _asvrpawn)
    (`AudioComponent.FadeOut` (`self.AmbientSound`) 3.0 0.0 "Linear")))

(fn `UserConstructionScript`)