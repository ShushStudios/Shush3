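; Breakable bathroom mirror actor, part of the pipe game, that shatters when struck by a hammer.
; An overlap on the Mirror component checks the other component for the "Hammer" tag.
; On a match it spawns a bathroom pipe piece and four differently shaped glass shards at preset point components, then destroys itself.
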(event `self.Mirror.OnComponentBeginOverlap`
  (params (OverlappedComponent :type "PrimitiveComponent Object Reference") (OtherActor :type "Actor Object Reference") (OtherComp :type "PrimitiveComponent Object Reference") (OtherBodyIndex :type Integer) (bFromSweep :type Boolean) (SweepResult :type "HitResult Structure (by ref)"))
  (if (`ActorComponent.ComponentHasTag` OtherComp "Hammer")
    (`self.SpawnObjects`)
    (`self.K2_DestroyActor`)))

(event `SpawnObjects`
  (`|SpawnActorFromClass` "/Game/assets/haydon/house/bathroom/assets/haydon/house/bathroom/Blueprints/PipeGameFiles/Blueprints/BP_BathroomPipe6.BP_BathroomPipe6_C" (`SceneComponent.GetSocketTransform` (`self.PipePoint`) "None" "RTS_World") "Undefined" "OverrideRootScale" null null)
  (`|SpawnActorFromClass` "/Game/assets/haydon/house/bathroom/assets/haydon/house/bathroom/Blueprints/PipeGameFiles/Blueprints/BP_BathroomGlassAngular.BP_BathroomGlassAngular_C" (`SceneComponent.GetSocketTransform` (`self.AngularPoint`) "None" "RTS_World") "Undefined" "OverrideRootScale" null null)
  (`|SpawnActorFromClass` "/Game/assets/haydon/house/bathroom/assets/haydon/house/bathroom/Blueprints/PipeGameFiles/Blueprints/BP_BathroomGlassEqualateral.BP_BathroomGlassEqualateral_C" (`SceneComponent.GetSocketTransform` (`self.EqualateralPoint`) "None" "RTS_World") "Undefined" "OverrideRootScale" null null)
  (`|SpawnActorFromClass` "/Game/assets/haydon/house/bathroom/assets/haydon/house/bathroom/Blueprints/PipeGameFiles/Blueprints/BP_BathroomGlassLarge.BP_BathroomGlassLarge_C" (`SceneComponent.GetSocketTransform` (`self.LargePoint`) "None" "RTS_World") "Undefined" "OverrideRootScale" null null)
  (`|SpawnActorFromClass` "/Game/assets/haydon/house/bathroom/assets/haydon/house/bathroom/Blueprints/PipeGameFiles/Blueprints/BP_BathroomGlassSmall.BP_BathroomGlassSmall_C" (`SceneComponent.GetSocketTransform` (`self.SmallPoint`) "None" "RTS_World") "Undefined" "OverrideRootScale" null null))

(fn `UserConstructionScript`)