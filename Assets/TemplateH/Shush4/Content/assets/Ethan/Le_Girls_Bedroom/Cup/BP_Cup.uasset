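; BP_Cup is a hittable doll head target that scores when struck by a component tagged ArmHammer.
; An overlap on DollHeadCollision sets Hit, hides DollHead, increments Score and prints it.
; Tick re-shows the head through a 3-second Delay while Hit is true, and Hit is never cleared, so that delay keeps cycling after the first strike.
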(event `self.ReceiveTick`
  (params (DeltaSeconds :type "Float (single-precision)"))
  (if (`self.Hit`)
    (`KismetSystemLibrary.Delay` 3.0)
    (`SceneComponent.SetVisibility` (`self.DollHead`) true false)))

(event `self.DollHeadCollision.OnComponentBeginOverlap`
  (params (OverlappedComponent :type "PrimitiveComponent Object Reference") (OtherActor :type "Actor Object Reference") (OtherComp :type "PrimitiveComponent Object Reference") (OtherBodyIndex :type Integer) (bFromSweep :type Boolean) (SweepResult :type "HitResult Structure (by ref)"))
  (if (`ActorComponent.ComponentHasTag` OtherComp "ArmHammer")
    (set `self.Hit` true)
    (`SceneComponent.SetVisibility` (`self.DollHead`) false false)
    (bind _output_get (set `self.Score` (+ (`self.Score`) 1)))
    (`KismetSystemLibrary.PrintString` (`KismetStringLibrary.Conv_IntToString` _output_get))))

(fn `UserConstructionScript`)