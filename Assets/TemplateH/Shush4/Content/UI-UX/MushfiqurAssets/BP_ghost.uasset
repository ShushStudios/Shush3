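; Ghost actor for a window jumpscare that briefly appears alongside an explosion sound and a flickering outside light.
; WIndowJumpscare plays the 2D sound, unhides the actor, starts FlickerLight, then hides the actor after a short delay.
; FlickerLight toggles OutsideLight visibility through chained delays, so it keeps running after the ghost disappears and finishes with the light off.
; Nothing in this Blueprint triggers the scare itself.
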(event `Show ghost`
  (`self.SetActorHiddenInGame` false))

(event `Hide ghost`
  (`self.SetActorHiddenInGame` true))

(event `Flicker Light`
  (bind _outside_light (`self.Outside light`))
  (`SceneComponent.SetVisibility` _outside_light true false)
  (`KismetSystemLibrary.Delay` 0.5)
  (`SceneComponent.SetVisibility` _outside_light true false)
  (`KismetSystemLibrary.Delay` 0.3)
  (`SceneComponent.SetVisibility` _outside_light false false)
  (`KismetSystemLibrary.Delay` 0.4)
  (`SceneComponent.SetVisibility` _outside_light false false)
  (`KismetSystemLibrary.Delay` 0.3)
  (`SceneComponent.SetVisibility` _outside_light true false)
  (`KismetSystemLibrary.Delay` 2.0)
  (`SceneComponent.SetVisibility` _outside_light false false))

(event `WIndow Jumpscare`
  (`GameplayStatics.PlaySound2D` "/Game/StarterContent/Audio/Explosion01.Explosion01" 1.0 1.0 0.4 null null false)
  (`self.Show ghost`)
  (`self.Flicker Light`)
  (`KismetSystemLibrary.Delay` 1.5)
  (`self.Hide ghost`))

(fn `UserConstructionScript`)