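; BP_ghost_scary is an actor whose Ghost component periodically appears and disappears during play.
; BeginPlay runs a hard-coded, unlooped chain of visibility toggles separated by 30-second delays, without propagating to child components.
; The ghost shows five times, then stays hidden after the final toggle at about four and a half minutes.
; The overlap event and construction script are empty.
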(event `self.ReceiveBeginPlay`
  (`SceneComponent.SetVisibility` (`self.Ghost`) true false)
  (`KismetSystemLibrary.Delay` 30.0)
  (`SceneComponent.SetVisibility` (`self.Ghost`) false false)
  (`KismetSystemLibrary.Delay` 30.0)
  (`SceneComponent.SetVisibility` (`self.Ghost`) true false)
  (`KismetSystemLibrary.Delay` 30.0)
  (`SceneComponent.SetVisibility` (`self.Ghost`) false false)
  (`KismetSystemLibrary.Delay` 30.0)
  (`SceneComponent.SetVisibility` (`self.Ghost`) true false)
  (`KismetSystemLibrary.Delay` 30.0)
  (`SceneComponent.SetVisibility` (`self.Ghost`) false false)
  (`KismetSystemLibrary.Delay` 30.0)
  (`SceneComponent.SetVisibility` (`self.Ghost`) true false)
  (`KismetSystemLibrary.Delay` 30.0)
  (`SceneComponent.SetVisibility` (`self.Ghost`) false false)
  (`KismetSystemLibrary.Delay` 30.0)
  (`SceneComponent.SetVisibility` (`self.Ghost`) true false)
  (`KismetSystemLibrary.Delay` 30.0)
  (`SceneComponent.SetVisibility` (`self.Ghost`) false false))

(fn `UserConstructionScript`)