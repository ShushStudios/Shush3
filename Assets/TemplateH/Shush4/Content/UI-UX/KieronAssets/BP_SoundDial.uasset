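; BP_SoundDial is a sound meter actor with a rotating dial and an overlap-driven highlight.
; Actor overlap toggles custom depth rendering on SoundOmeter to show or hide its outline.
; As a movement test, BeginPlay drives the SoundDialMove timeline, which lerps the SoundDial's relative roll through a negative arc.
; A FlipFlop provides a reverse branch, but BeginPlay fires once, so only the forward play runs.
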(event `self.ReceiveActorBeginOverlap`
  (params (OtherActor :type "Actor Object Reference"))
  ;[1 1 1] OUTLINE SETUP
  (`PrimitiveComponent.SetRenderCustomDepth` (`self.SoundOmeter`) true))

(event `self.ReceiveActorEndOverlap`
  (params (OtherActor :type "Actor Object Reference"))
  ;[1 1 1] OUTLINE SETUP
  (`PrimitiveComponent.SetRenderCustomDepth` (`self.SoundOmeter`) false))

(event `self.ReceiveBeginPlay`
  ;[1 1 1] Added to test movement
  (`/Engine/EditorBlueprintResources/StandardMacros.FlipFlop`
    (:`A`
      (bind (_direction _sounddial_track) (`Timeline|SoundDial Move` :`NewTime` (`self.SoundDial Rotation`) :!label _label)
        (:`Update`
          (`SceneComponent.K2_SetRelativeRotation` (`self.SoundDial`) (`KismetMathLibrary.MakeRotator` (`KismetMathLibrary.Lerp` 0.0 -159.0 _sounddial_track)) false false))))
    (:`B`
      (goto _label :!via `Reverse`))))

(fn `UserConstructionScript`)