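; Bathroom pipe puzzle Blueprint where six pipe pieces are placed into trigger slots to clear a blocking component.
; Each trigger checks the overlapping component's tag, destroys that actor, reveals its built-in pipe and sets a placed flag, enabling collision on all but Pipe6.
; Completion is checked only when the GrabComponent is grabbed; with all six flags set, Block is hidden and loses collision.
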(event `self.ReceiveBeginPlay`)

(event `CheckPipes`
  (if (and (and (`self.Pipe1Placed`) (and (`self.Pipe6Placed`) (`self.Pipe5Placed`))) (and (and (`self.Pipe4Placed`) (`self.Pipe3Placed`)) (`self.Pipe2Placed`)))
    (`KismetSystemLibrary.PrintString` "pipes")
    (`SceneComponent.SetVisibility` (`self.Block`) false false)
    (`PrimitiveComponent.SetCollisionEnabled` (`self.Block`) "NoCollision")))

(event `self.Pipe1Trigger.OnComponentBeginOverlap`
  (params (OverlappedComponent :type "PrimitiveComponent Object Reference") (OtherActor :type "Actor Object Reference") (OtherComp :type "PrimitiveComponent Object Reference") (OtherBodyIndex :type Integer) (bFromSweep :type Boolean) (SweepResult :type "HitResult Structure (by ref)"))
  (if (`ActorComponent.ComponentHasTag` OtherComp "Pipe1")
    (`self.K2_DestroyActor` OtherActor)
    (`SceneComponent.SetVisibility` (`self.Pipe1`) true false)
    (`PrimitiveComponent.SetCollisionEnabled` (`self.Pipe1`) "QueryAndPhysics")
    (set `self.Pipe1Placed` true)))

(event `self.Pipe2Trigger.OnComponentBeginOverlap`
  (params (OverlappedComponent :type "PrimitiveComponent Object Reference") (OtherActor :type "Actor Object Reference") (OtherComp :type "PrimitiveComponent Object Reference") (OtherBodyIndex :type Integer) (bFromSweep :type Boolean) (SweepResult :type "HitResult Structure (by ref)"))
  (if (`ActorComponent.ComponentHasTag` OtherComp "Pipe2")
    (`self.K2_DestroyActor` OtherActor)
    (`SceneComponent.SetVisibility` (`self.Pipe2`) true false)
    (`PrimitiveComponent.SetCollisionEnabled` (`self.Pipe2`) "QueryAndPhysics")
    (set `self.Pipe2Placed` true)))

(event `self.Pipe3Trigger.OnComponentBeginOverlap`
  (params (OverlappedComponent :type "PrimitiveComponent Object Reference") (OtherActor :type "Actor Object Reference") (OtherComp :type "PrimitiveComponent Object Reference") (OtherBodyIndex :type Integer) (bFromSweep :type Boolean) (SweepResult :type "HitResult Structure (by ref)"))
  (if (`ActorComponent.ComponentHasTag` OtherComp "Pipe3")
    (`self.K2_DestroyActor` OtherActor)
    (`SceneComponent.SetVisibility` (`self.Pipe3`) true false)
    (`PrimitiveComponent.SetCollisionEnabled` (`self.Pipe3`) "QueryAndPhysics")
    (set `self.Pipe3Placed` true)))

(event `self.Pipe4Trigger.OnComponentBeginOverlap`
  (params (OverlappedComponent :type "PrimitiveComponent Object Reference") (OtherActor :type "Actor Object Reference") (OtherComp :type "PrimitiveComponent Object Reference") (OtherBodyIndex :type Integer) (bFromSweep :type Boolean) (SweepResult :type "HitResult Structure (by ref)"))
  (if (`ActorComponent.ComponentHasTag` OtherComp "Pipe4")
    (`self.K2_DestroyActor` OtherActor)
    (`SceneComponent.SetVisibility` (`self.Pipe4`) true false)
    (`PrimitiveComponent.SetCollisionEnabled` (`self.Pipe4`) "QueryAndPhysics")
    (set `self.Pipe4Placed` true)))

(event `self.Pipe5Trigger.OnComponentBeginOverlap`
  (params (OverlappedComponent :type "PrimitiveComponent Object Reference") (OtherActor :type "Actor Object Reference") (OtherComp :type "PrimitiveComponent Object Reference") (OtherBodyIndex :type Integer) (bFromSweep :type Boolean) (SweepResult :type "HitResult Structure (by ref)"))
  (if (`ActorComponent.ComponentHasTag` OtherComp "Pipe5")
    (`self.K2_DestroyActor` OtherActor)
    (`SceneComponent.SetVisibility` (`self.Pipe5`) true false)
    (`PrimitiveComponent.SetCollisionEnabled` (`self.Pipe5`) "QueryAndPhysics")
    (set `self.Pipe5Placed` true)))

(event `self.Pipe6Trigger.OnComponentBeginOverlap`
  (params (OverlappedComponent :type "PrimitiveComponent Object Reference") (OtherActor :type "Actor Object Reference") (OtherComp :type "PrimitiveComponent Object Reference") (OtherBodyIndex :type Integer) (bFromSweep :type Boolean) (SweepResult :type "HitResult Structure (by ref)"))
  (if (`ActorComponent.ComponentHasTag` OtherComp "Pipe6")
    (`self.K2_DestroyActor` OtherActor)
    (`SceneComponent.SetVisibility` (`self.Pipe6`) true false)
    (`PrimitiveComponent.SetCollisionEnabled` (`self.Pipe6`) "NoCollision")
    (set `self.Pipe6Placed` true)))

(event `self.GrabComponent.OnGrabbed`
  (`self.CheckPipes`))

(fn `UserConstructionScript`)