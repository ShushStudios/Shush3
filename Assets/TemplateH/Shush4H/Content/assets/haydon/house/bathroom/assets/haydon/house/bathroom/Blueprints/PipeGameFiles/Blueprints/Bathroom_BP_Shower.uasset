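; Bathroom shower for the pipe game, whose pipe and shower head can be grabbed loose.
; At start the pipe is scaled up with physics off.
; The first pipe grab spawns a separate Bathroom_BP_Pipe at its location, hides the original and drops the shower head into physics, with CanPickUp guarding against repeats.
; Grabbing the shower head also turns on its physics.
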(event `self.ReceiveBeginPlay`
  (`SceneComponent.SetRelativeScale3D` (`self.Pipe`) (3.0 3.0 3.0))
  (`PrimitiveComponent.SetSimulatePhysics` (`self.Pipe`) false))

(event `self.GrabComponentPipe.OnGrabbed`
  (bind _pipe (`self.Pipe`))
  (if (not (`self.canPickUp`))
    (`|SpawnActorFromClass` "/Game/assets/haydon/house/bathroom/assets/haydon/house/bathroom/Blueprints/PipeGameFiles/Blueprints/Bathroom_BP_Pipe.Bathroom_BP_Pipe_C" (`KismetMathLibrary.Conv_VectorToTransform` (`SceneComponent.K2_GetComponentLocation` _pipe)) "Undefined" "OverrideRootScale" null null)
    (`SceneComponent.SetVisibility` _pipe false false)
    (`PrimitiveComponent.SetSimulatePhysics` (`self.ShowerHead`) true)
    (set `self.canPickUp` true)))

(event `self.GrabComponentShower.OnGrabbed`
  (`PrimitiveComponent.SetSimulatePhysics` (`self.ShowerHead`) true))

(fn `UserConstructionScript`)